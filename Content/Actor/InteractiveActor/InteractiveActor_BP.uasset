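; Interactive actor Blueprint that shows a configurable static mesh and provides events to add or remove a highlight outline.
; BeginPlay assigns the mesh; CreateOutline spawns a duplicate mesh component at the same world transform with a dynamic outline material on slot 0, parameterized by color and scale.
; DeleteOutline destroys that duplicate, with the NeedOutline flag preventing repeated creation.
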(event Custom|Create%20Outline
  ;[1 1 1] 设置高亮轮廓
  (if (Variables|Default|GetNeed%20Outline)
    (bind _returnvalue (AddComponent|AddStaticMeshComponent true (Transformation|GetWorldTransform (Variables|Default|GetStaticMesh))))
    (bind _output_get (Variables|Default|SetStaticMeshComp _returnvalue))
    (Components|StaticMesh|SetStaticMesh _output_get (Variables|Default|GetMesh))
    (bind _returnvalue_2 (Rendering|Material|CreateDynamicMaterialInstance _output_get 0 "/Game/Meshes/M_Outline_Inst.M_Outline_Inst" "None" :!class /Script/Engine.PrimitiveComponent))
    (Rendering|Material|SetVectorParameterValue _returnvalue_2 "Color" (Variables|Default|GetColor) :!class /Script/Engine.MaterialInstanceDynamic)
    (Rendering|Material|SetScalarParameterValue _returnvalue_2 "Scale" (Variables|Default|GetScale) :!class /Script/Engine.MaterialInstanceDynamic)
    (Variables|Default|SetNeed%20Outline false)))

(event Custom|Delete%20Outline
  (bind _staticmeshcomp (Variables|Default|GetStaticMeshComp))
  ;[1 1 1] 删除高亮轮廓
  (Utilities|IsValid _staticmeshcomp
    (:Is%20Valid
      (Components|DestroyComponent _staticmeshcomp)
      (Variables|Default|SetNeed%20Outline true))))

(event EventBeginPlay
  ;[1 1 1] 设置物体实例
  (Components|StaticMesh|SetStaticMesh (Variables|Default|GetStaticMesh) (Variables|Default|GetMesh)))

(event Collision|EventActorBeginOverlap
  (params (OtherActor :type Actor%20Object%20Reference)))

(event EventTick
  (params (DeltaSeconds :type Float%20%28single-precision%29)))

(fn ConstructionScript)